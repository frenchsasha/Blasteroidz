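; Player ship character for an asteroid shooter that fires projectiles, grapples asteroids and reports its destruction to the game mode to update lives.
; Fire spawns a projectile ahead of the ship, throttled by a DoOnce and short delay.
; Grapple sphere-traces forward; while held after a hit, Tick spawns an impact point at the asteroid every frame and attaches the cable to the asteroid.
; Tick also draws a debug line showing velocity.
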(event OnComponentBeginOverlap(CapsuleComponent)
  (params (OverlappedComponent :type Primitive%20Component%20Object%20Reference) (OtherActor :type Actor%20Object%20Reference) (OtherComp :type Primitive%20Component%20Object%20Reference) (OtherBodyIndex :type Integer) (bFromSweep :type Boolean) (SweepResult :type Hit%20Result%20Structure%20%28by%20ref%29)))

(event Custom|Death
  (params (DestroyedActor :type Actor%20Object%20Reference))
  (Default|UpdateLives (Variables|Default|GetREF_GameMode)))

(event EventBeginPlay
  (Utilities|FlowControl|Sequence
    (:then_0
      (bind _asblasteroidz_game_mode (Utilities|Casting|CastToBlasteroidzGameMode (Game|GetGameMode)))
      (Variables|Default|SetREF_GameMode _asblasteroidz_game_mode))
    (:then_1
      (Game|BindEventtoOnDestroyed (delegate Custom|Death)))))

(event EventTick
  (params (DeltaSeconds :type Float%20%28single-precision%29))
  (bind _returnvalue (Transformation|GetActorLocation))
  ;[1 1 1] Visualize Velocity
  (Rendering|Debug|DrawDebugLine _returnvalue (+ _returnvalue (Variables|/Script/Engine.MovementComponent|GetVelocity (Variables|Character|GetCharacterMovement))) "(R=0.000000,G=1.000000,B=0.001847,A=1.000000)" 0.0 5.0)
  ;[1 1 1] Unide Cable
  (if (stale Input|ActionEvents|InputActionGrapple _output_get)
    (Development|SetHiddeninGame (Variables|Default|GetCable) false false)
    (bind _asasteroid_bp (Utilities|Casting|CastToAsteroid_BP (.HitActor (Collision|BreakHitResult (stale Input|ActionEvents|InputActionGrapple _outhit)))))
    (bind _returnvalue_2 (Game|SpawnActorfromClass "/Game/ImpactPoint.ImpactPoint_C" (Math|Conversions|ToTransform(Vector) (Transformation|GetActorLocation _asasteroid_bp)) "Undefined" 0 0))
    (Variables|Default|SetGrapplingActor _returnvalue_2)
    (Class|CableComponent|SetAttachEndto (Variables|Default|GetCable) _asasteroid_bp "None" "None")))

(event Input|ActionEvents|InputActionFire
  (params (Key :type Key%20Structure))
  (bind _returnvalue (Transformation|GetActorForwardVector))
  ;[1 1 1] Fire
  (:Pressed
    (Utilities|FlowControl|DoOnce false :!label _label
      (:Completed
        (Game|SpawnActorfromClass "/Game/ProjectileBaseBP.ProjectileBaseBP_C" (Math|Transform|MakeTransform (+ (Transformation|GetActorLocation) (* _returnvalue 1e+02)) (Math|Conversions|RotationFromXVector _returnvalue) "1,1,1") "AlwaysSpawn" 0 0)
        (Utilities|FlowControl|Delay 0.25)
        (goto _label Reset)))))

(event Input|ActionEvents|InputActionGrapple
  (params (Key :type Key%20Structure))
  (bind _returnvalue (Transformation|GetActorLocation))
  (:Pressed
    ;[1 1 1] Search and Grab Asteroid
    (bind (_outhit _returnvalue_2) (Collision|SphereTraceByChannel _returnvalue (+ _returnvalue (* (Transformation|GetActorForwardVector) (Variables|Default|GetGrappleDistance))) 2e+01 "TraceTypeQuery1" false 0 "None"))
    (if _returnvalue_2
      (Variables|Default|SetImpact%20Point (.ImpactPoint (Collision|BreakHitResult _outhit)))
      (bind _output_get (Variables|Default|SetGrappleConnected true))
      (Variables|Default|SetHit%20Actor (.HitActor (Collision|BreakHitResult _outhit)))))
  (:Released
    ;[1 1 1] Hide Grapple on Release
    (Variables|Default|SetGrappleConnected false)
    (Development|SetHiddeninGame (Variables|Default|GetCable) true false)))

(fn ConstructionScript)