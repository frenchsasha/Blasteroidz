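; BP_Shooter is a mouse-aimed shooter that fires BP_Projectile actors, with Q handing possession back to the ThirdPersonCharacter cached at BeginPlay.
; Tick rotates an Arrow using a far point along the deprojected mouse ray as its direction vector.
; Left click spawns one projectile from the Arrow with that rotation.
; Holding right click fires immediately and repeats through a self-rescheduling Interval timer controlled by a gate.
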(event Custom|AutoFire
  (bind _returnvalue (Game|GetPlayerController 0))
  (bind (_worldlocation _worlddirection) (Game|Player|ConvertMouseLocationToWorldSpace _returnvalue))
  (Utilities|FlowControl|Gate true
    (:Exit
      (Utilities|Time|SetTimerbyEvent (delegate Custom|AutoFire) (Variables|Default|GetInterval))
      (Game|SpawnActorfromClass "/Game/AdvancedShieldSystem/Blueprints/BP_Projectile.BP_Projectile_C" (Math|Transform|MakeTransform (Transformation|GetWorldLocation (Variables|Default|GetArrow)) (Math|Conversions|RotationFromXVector (+ _worldlocation (* _worlddirection 1e+04))) "1,1,1") "Undefined" 0 0))))

(event EventBeginPlay
  (bind _asthird_person_character (Utilities|Casting|CastToThirdPersonCharacter (Game|Player|GetPlayerPawn 0)))
  (Variables|Default|SetCharacterBP _asthird_person_character))

(event EventTick
  (params (DeltaSeconds :type Float%20%28single-precision%29))
  (bind _returnvalue (Game|GetPlayerController 0))
  (bind (_worldlocation _worlddirection) (Game|Player|ConvertMouseLocationToWorldSpace _returnvalue))
  (Transformation|SetWorldRotation (Variables|Default|GetArrow) (Math|Conversions|RotationFromXVector (+ _worldlocation (* _worlddirection 1e+04))) false false))

(event Input|MouseEvents|LeftMouseButton
  (params (Key :type Key%20Structure))
  (bind _returnvalue (Game|GetPlayerController 0))
  (bind (_worldlocation _worlddirection) (Game|Player|ConvertMouseLocationToWorldSpace _returnvalue))
  (:Pressed
    (Game|SpawnActorfromClass "/Game/AdvancedShieldSystem/Blueprints/BP_Projectile.BP_Projectile_C" (Math|Transform|MakeTransform (Transformation|GetWorldLocation (Variables|Default|GetArrow)) (Math|Conversions|RotationFromXVector (+ _worldlocation (* _worlddirection 1e+04))) "1,1,1") "Undefined" 0 0)))

(event Input|MouseEvents|RightMouseButton
  (params (Key :type Key%20Structure))
  (bind _returnvalue (Game|GetPlayerController 0))
  (bind (_worldlocation _worlddirection) (Game|Player|ConvertMouseLocationToWorldSpace _returnvalue))
  (:Pressed
    (Utilities|FlowControl|Sequence
      (:then_0
        (Utilities|FlowControl|Gate true) ; enters at Open
      )
      (:then_1
        (Utilities|Time|SetTimerbyEvent (delegate Custom|AutoFire) (Variables|Default|GetInterval))
        (Game|SpawnActorfromClass "/Game/AdvancedShieldSystem/Blueprints/BP_Projectile.BP_Projectile_C" (Math|Transform|MakeTransform (Transformation|GetWorldLocation (Variables|Default|GetArrow)) (Math|Conversions|RotationFromXVector (+ _worldlocation (* _worlddirection 1e+04))) "1,1,1") "Undefined" 0 0))))
  (:Released
    (Utilities|FlowControl|Gate true) ; enters at Close
  ))

(event Input|KeyboardEvents|Q
  (params (Key :type Key%20Structure))
  (:Pressed
    (Pawn|Possess (Game|GetPlayerController 0) (Variables|Default|GetCharacterBP))))

(fn ConstructionScript)