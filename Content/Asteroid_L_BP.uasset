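; Large asteroid actor that drifts under physics and drives the pull of the player ship's grapple.
; BeginPlay randomizes its rotation and caches the player ship.
; Each Tick applies a randomized, horizontal acceleration within a cone around the mesh's forward vector.
; While the grapple is connected, every instance accelerates the ship's HitActor toward the ship, scaled by distance over MaxDist, without checking that it is the hit actor.
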(event EventBeginPlay
  (Transformation|SetActorRotation (Math|Random|RandomRotator true))
  (bind _asplayer_ship_character_bp (Utilities|Casting|CastToPlayerShipCharacterBP (Game|Player|GetPlayerPawn 0)))
  (Variables|Default|SetAs%20Player%20Ship%20Character%20BP _asplayer_ship_character_bp))

(event Collision|EventActorBeginOverlap
  (params (OtherActor :type Actor%20Object%20Reference)))

(event EventTick
  (params (DeltaSeconds :type Float%20%28single-precision%29))
  (bind _staticmesh (Variables|Default|GetStaticMesh))
  (bind _returnvalue (Math|Vector|GetForwardVector _staticmesh))
  (bind _returnvalue_2 (Math|Random|RandomUnitVectorinConeinDegrees _returnvalue 45.0))
  (bind (_x _y) (Math|Vector|BreakVector _returnvalue_2))
  (Physics|AddForce (Variables|Default|GetStaticMesh self) (* (Math|Vector|MakeVector _x _y 0.0) (* 2e+02 (Math|Float|MapRangeClamped (Math|Random|RandomFloat) 0.0 1.0 0.2 1.0))) "None" true)
  (if (Variables|/Game/PlayerShipCharacterBP.PlayerShipCharacterBP_C|GetGrappleConnected (Variables|Default|GetAs%20Player%20Ship%20Character%20BP))
    (Physics|AddForce (Actor|GetComponentbyClass (Variables|/Game/PlayerShipCharacterBP.PlayerShipCharacterBP_C|GetHit%20Actor (Variables|Default|GetAs%20Player%20Ship%20Character%20BP)) "/Script/Engine.StaticMeshComponent") (* (* (Math|Vector|Normalize (- (Transformation|GetActorLocation (Variables|Default|GetAs%20Player%20Ship%20Character%20BP)) (.Origin (Collision|GetActorBounds (Variables|/Game/PlayerShipCharacterBP.PlayerShipCharacterBP_C|GetHit%20Actor (Variables|Default|GetAs%20Player%20Ship%20Character%20BP)) false false)))) 15.0) (/ (Math|Vector|Distance(Vector) (.Origin (Collision|GetActorBounds (Variables|/Game/PlayerShipCharacterBP.PlayerShipCharacterBP_C|GetHit%20Actor (Variables|Default|GetAs%20Player%20Ship%20Character%20BP)) false false)) (Transformation|GetActorLocation (Variables|Default|GetAs%20Player%20Ship%20Character%20BP))) (Variables|Default|GetMaxDist))) "None" true)))

(fn ConstructionScript)